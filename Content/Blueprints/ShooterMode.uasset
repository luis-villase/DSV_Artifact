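; ShooterMode holds the shooter's game rules, driving enemy spawning and player respawn.
; On BeginPlay it plays the Breakdown sound and starts a looping timer on the first BasicEnemySpawner found, calling SpawnBasicEnemy at BasicEPS times per second.
; RespawnPlayer destroys every BasicEnemyCharacter, spawns a new PlayerCharacter at PlayerSpawnTransform and has player controller 0 possess it.
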(event Custom|RespawnPlayer
  (bind _outactors (Actor|GetAllActorsOfClass "/Game/Blueprints/BasicEnemyCharacter.BasicEnemyCharacter_C"))
  (for _array_element _outactors
    (Actor|DestroyActor _array_element))
  (bind _returnvalue (Game|SpawnActorfromClass "/Game/Blueprints/PlayerCharacter.PlayerCharacter_C" (Variables|Default|GetPlayerSpawnTransform) "Undefined" 0 0))
  (Pawn|Possess (Game|GetPlayerController 0) _returnvalue))

(event EventBeginPlay
  (Audio|PlaySound2D "/Game/Audio/Breakdown.Breakdown" 0.7 1.0 0.0 0 0)
  (bind _outactors (Actor|GetAllActorsOfClass "/Game/Blueprints/BasicEnemySpawner.BasicEnemySpawner_C"))
  (bind _output_get (Variables|Default|SetBasicEnemySpawner (Utilities|Array|Get(acopy) _outactors)))
  (Utilities|Time|SetTimerbyFunctionName _output_get "SpawnBasicEnemy" (/ 1.0 (Variables|Default|GetBasicEPS)) true))

(fn ConstructionScript)