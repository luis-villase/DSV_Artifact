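; Bullet projectile actor that damages what it overlaps and then destroys itself.
; On overlap with an IDamagable actor not tagged "None", it randomly boosts its negative Damage for a critical hit, sends it via AffectHealthMessage and plays a random impact sound.
; Non-damagable overlaps destroy it immediately, while damagable actors tagged "None" leave it intact.
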(event Collision|EventActorBeginOverlap
  (params (OtherActor :type Actor%20Object%20Reference))
  (Variables|Default|SetBulletPos (Transformation|GetWorldLocation (Variables|Default|Get50bmg_bullet)))
  (if (Utilities|DoesObjectImplementInterface OtherActor "/Game/Blueprints/IDamagable.IDamagable_C")
    (if (not (Actor|ActorHasTag OtherActor "None"))
      (if (> (Math|Random|RandomInteger 5) 3)
        (Variables|Default|SetDamage (* (Variables|Default|GetDamage) 2.5)))
      (Class|IDamagable|AffectHealth(Message) OtherActor (Variables|Default|GetDamage))
      (switch int (Math|Random|RandomInteger 7)
        (:Default
          (Audio|PlaySoundatLocation "/Game/Audio/hit7.hit7" (Variables|Default|GetBulletPos) "0, 0, 0" 1.0 1.0 0.0 0 0 0))
        (:0
          (Audio|PlaySoundatLocation "/Game/Audio/hit1.hit1" (Variables|Default|GetBulletPos) "0, 0, 0" 1.0 1.0 0.0 0 0 0))
        (:1
          (Audio|PlaySoundatLocation "/Game/Audio/hit2.hit2" (Variables|Default|GetBulletPos) "0, 0, 0" 1.0 1.0 0.0 0 0 0))
        (:2
          (Audio|PlaySoundatLocation "/Game/Audio/hit4.hit4" (Variables|Default|GetBulletPos) "0, 0, 0" 1.0 1.0 0.0 0 0 0))
        (:3
          (Audio|PlaySoundatLocation "/Game/Audio/hit4.hit4" (Variables|Default|GetBulletPos) "0, 0, 0" 1.0 1.0 0.0 0 0 0))
        (:4
          (Audio|PlaySoundatLocation "/Game/Audio/hit5.hit5" (Variables|Default|GetBulletPos) "0, 0, 0" 1.0 1.0 0.0 0 0 0))
        (:5
          (Audio|PlaySoundatLocation "/Game/Audio/hit6.hit6" (Variables|Default|GetBulletPos) "0, 0, 0" 1.0 1.0 0.0 0 0 0)))
      (Variables|Default|SetDamage -2e+01)
      (Actor|DestroyActor :!label _label))
    (else
      (goto _label))))

(fn ConstructionScript)