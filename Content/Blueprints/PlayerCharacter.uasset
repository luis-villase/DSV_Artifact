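; Player character for a shooter with twin-stick style controls, spawning its gun on a mesh socket and creating the HUD at start.
; Axis inputs drive world-axis and forward movement, controller yaw, and stick aiming that pulls the gun trigger past a deadzone.
; The Fire action loops shots through a Gate and retriggerable delay at RPS rate.
; On death it disables input, then asks ShooterMode to respawn and destroys itself and its gun.
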(event EventBeginPlay
  (bind _mesh (Variables|Character|GetMesh))
  (Utilities|FlowControl|Sequence
    (:then_0
      (bind _returnvalue (Game|SpawnActorfromClass "/Game/Blueprints/Gun.Gun_C" (Transformation|GetWorldTransform _mesh) "Undefined" 0 0))
      (bind _output_get (Variables|Default|SetGun _returnvalue))
      (Transformation|AttachComponentToComponent _output_get _mesh "GunSocket" "KeepWorld" "KeepWorld" "KeepWorld" true))
    (:then_1
      (bind _asshooter_mode (Utilities|Casting|CastToShooterMode (Game|GetGameMode)))
      (bind _output_get_2 (Variables|Default|SetGameMode _asshooter_mode))
      (Variables|/Game/Blueprints/ShooterMode.ShooterMode_C|SetPlayerSpawnTransform _output_get_2 (Transformation|GetActorTransform)))
    (:then_2
      (bind _returnvalue_2 (UserInterface|CreateWidget "/Game/Blueprints/HUD.HUD_C"))
      (UserInterface|Viewport|AddtoViewport _returnvalue_2 0))))

(event EventAffectHealth
  (params (Delta :type Float%20%28single-precision%29))
  (Class|BaseCharacter|CalculateHealth Delta)
  (if (Variables|Default|GetisDead)
    (Input|DisableInput (Game|GetPlayerController 0) 0)
    (Utilities|FlowControl|Delay 3.0)
    (bind _asshooter_mode (Utilities|Casting|CastToShooterMode (Game|GetGameMode)))
    (Default|RespawnPlayer _asshooter_mode)
    (Actor|DestroyActor (Variables|Default|GetGun))))

(event Input|ActionEvents|InputActionFire
  (params (Key :type Key%20Structure))
  ;[1 1 1] Mouse Fire
  (:Pressed
    (Utilities|FlowControl|Sequence
      (:then_0
        (goto _label Open))
      (:then_1
        (Utilities|FlowControl|Gate true :!label _label
          (:Exit
            (Utilities|FlowControl|Sequence
              (:then_0
                (Default|Fire (Variables|Default|GetGun)))
              (:then_1
                (Utilities|FlowControl|RetriggerableDelay (/ 1.0 (Variables|Default|GetRPS)))
                (goto _label))))))))
  (:Released
    (goto _label Close)))

(event Input|AxisEvents|InputAxisMoveUp
  (params (AxisValue :type Float%20%28single-precision%29))
  ;[1 1 1] Movement
  (Pawn|Input|AddMovementInput "1.000000, 0, 0" AxisValue false))

(event Input|AxisEvents|InputAxisMoveRight
  (params (AxisValue :type Float%20%28single-precision%29))
  ;[1 1 1] Movement
  (Pawn|Input|AddMovementInput "0.000000,1.000000, 0" AxisValue false))

(event Input|AxisEvents|InputAxisLookRight
  (params (AxisValue :type Float%20%28single-precision%29))
  (bind _gun (Variables|Default|GetGun))
  ;[1 1 1] Rotation
  (if (> (Math|Vector|VectorLength (Math|Vector|MakeVector (stale Input|AxisEvents|InputAxisLookUp AxisValue) AxisValue 0.0)) 0.25)
    (Pawn|SetControlRotation (Pawn|GetController) (Math|Conversions|RotationFromXVector (Math|Vector|MakeVector (stale Input|AxisEvents|InputAxisLookUp AxisValue) AxisValue 0.0)))
    (Default|PullTrigger _gun)
    (else
      (Default|Releaserigger _gun))))

(event Input|AxisEvents|InputAxisLookUp
  (params (AxisValue :type Float%20%28single-precision%29))
  (bind _gun (Variables|Default|GetGun))
  ;[1 1 1] Rotation
  (if (> (Math|Vector|VectorLength (Math|Vector|MakeVector AxisValue (stale Input|AxisEvents|InputAxisLookRight AxisValue) 0.0)) 0.25)
    (Pawn|SetControlRotation (Pawn|GetController) (Math|Conversions|RotationFromXVector (Math|Vector|MakeVector AxisValue (stale Input|AxisEvents|InputAxisLookRight AxisValue) 0.0)))
    (Default|PullTrigger _gun)
    (else
      (Default|Releaserigger _gun))))

(event Input|AxisEvents|InputAxisLookMove
  (params (AxisValue :type Float%20%28single-precision%29))
  ;[1 1 1] Keyboard Controls
  (Pawn|Input|AddControllerYawInput (* AxisValue 1.5)))

(event Input|AxisEvents|InputAxisMoveForward
  (params (AxisValue :type Float%20%28single-precision%29))
  ;[1 1 1] Keyboard Controls
  (Class|PawnMovementComponent|AddInputVector (Pawn|GetMovementComponent) (* (Transformation|GetActorForwardVector) AxisValue) false))

(fn ConstructionScript)