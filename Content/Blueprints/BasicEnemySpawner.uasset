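; Enemy spawner Blueprint that adds a random AI enemy inside its BasicSpawnVolume whenever its SpawnBasicEnemy event fires.
; It spawns only while the count of BasicEnemyCharacter actors in the world is below MaxBasicEnemies.
; A weighted random switch picks Basic, Dude, Vincent or Thug, with Thug half as likely as each of the others.
; SpawnAIFromClass places the pawn at a random point within the volume's bounds.
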(event Custom|SpawnBasicEnemy
  (bind _basicspawnvolume (Variables|Default|GetBasicSpawnVolume))
  (bind _basicspawnvolume_2 (Variables|Default|GetBasicSpawnVolume))
  (bind _basicspawnvolume_3 (Variables|Default|GetBasicSpawnVolume))
  (bind _basicspawnvolume_4 (Variables|Default|GetBasicSpawnVolume))
  (bind _outactors (Actor|GetAllActorsOfClass "/Game/Blueprints/BasicEnemyCharacter.BasicEnemyCharacter_C"))
  (if (< (Utilities|Array|Length _outactors) (Variables|Default|GetMaxBasicEnemies))
    (switch int (Math|Random|RandomInteger 7)
      (:0
        (AI|SpawnAIFromClass "/Game/Blueprints/BasicEnemyCharacter.BasicEnemyCharacter_C" 0 (Math|Random|RandomPointinBoundingBox (Transformation|GetWorldLocation _basicspawnvolume_2) (Components|Box|GetScaledBoxExtent _basicspawnvolume_2)) "0, 0, 0" false :!label _label))
      (:1
        (goto _label))
      (:2
        (AI|SpawnAIFromClass "/Game/Blueprints/DudeEnemyCharacter.DudeEnemyCharacter_C" 0 (Math|Random|RandomPointinBoundingBox (Transformation|GetWorldLocation _basicspawnvolume_3) (Components|Box|GetScaledBoxExtent _basicspawnvolume_3)) "0, 0, 0" false :!label _label_2))
      (:3
        (goto _label_2))
      (:4
        (AI|SpawnAIFromClass "/Game/Blueprints/VincentEnemyCharacter.VincentEnemyCharacter_C" 0 (Math|Random|RandomPointinBoundingBox (Transformation|GetWorldLocation _basicspawnvolume_4) (Components|Box|GetScaledBoxExtent _basicspawnvolume_4)) "0, 0, 0" false :!label _label_3))
      (:5
        (goto _label_3))
      (:6
        (AI|SpawnAIFromClass "/Game/Blueprints/ThugEnemyCharacter.ThugEnemyCharacter_C" 0 (Math|Random|RandomPointinBoundingBox (Transformation|GetWorldLocation _basicspawnvolume) (Components|Box|GetScaledBoxExtent _basicspawnvolume)) "0, 0, 0" false)))))

(fn ConstructionScript)