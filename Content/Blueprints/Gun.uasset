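; Gun is an automatic firearm Blueprint that fires Bullet actors for as long as its trigger is held.
; PullTrigger passes a DoOnce gate, fires immediately, then starts a looping timer on Fire at a rate set by RPS.
; Releaserigger clears that timer and resets the gate.
; Each Fire plays a rifle sound, attaches a muzzle flash and spawns a Bullet, all at ProjectileSpawnPt.
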(event Custom|PullTrigger
  (Utilities|FlowControl|DoOnce false
    (:Completed
      (CallFunction|Fire)
      (Utilities|Time|SetTimerbyFunctionName 0 "Fire" (/ 1.0 (Variables|Default|GetRPS)) true))))

(event Custom|Releaserigger
  (Utilities|Time|ClearTimerbyFunctionName 0 "Fire")
  (Utilities|FlowControl|DoOnce false) ; enters at Reset
)

(event Custom|Fire
  (bind _projectilespawnpt (Variables|Default|GetProjectileSpawnPt))
  (Audio|PlaySoundatLocation "/Game/Audio/404561__superphat__assaultrifle2.404561__superphat__assaultrifle2" (Transformation|GetWorldLocation (Variables|Default|GetProjectileSpawnPt)) "0, 0, 0" 0.6 1.0 0.0 0 0 0)
  (Effects|SpawnEmitterAttached "/Game/Weapons/M4A1/MuzzleFlash.MuzzleFlash" _projectilespawnpt "None")
  (Game|SpawnActorfromClass "/Game/Blueprints/Bullet.Bullet_C" (Transformation|GetWorldTransform _projectilespawnpt) "Undefined" 0 0))

(event EventBeginPlay)

(event Collision|EventActorBeginOverlap
  (params (OtherActor :type Actor%20Object%20Reference)))

(event EventTick
  (params (DeltaSeconds :type Float%20%28single-precision%29)))

(fn ConstructionScript)